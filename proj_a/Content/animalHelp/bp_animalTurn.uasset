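; Animal display Blueprint that continuously spins a group of skeletal mesh animals, including several low-poly animated chameleons.
; Each Tick calls TurnAnimal, which adds the same fixed local rotation to every listed mesh component.
; The rotation step is applied per frame without delta-time scaling, so spin speed follows frame rate.
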(event EventTick
  (params (DeltaSeconds :type Float%20%28single-precision%29))
  (CallFunction|TurnAnimal))

(fn ConstructionScript)

(fn TurnAnimal
  (Transformation|AddLocalRotation (Variables|Default|Getlowpoly_animated_chamaleon_game_ready1) "0.000000,-3.000000,0.000000" false false))