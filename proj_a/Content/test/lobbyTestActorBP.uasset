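; Lobby test actor that loops a Fox and a Giraffe component through continuous movement.
; Each Tick pushes the Fox along FoxArrow's forward vector, and Check snaps it back to a fixed relative start once its Y passes the Box.
; The Giraffe moves along world X and, past a threshold, jumps back with a random Y.
; Both use fixed per-frame steps without delta time, so speed depends on frame rate.
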(event EventBeginPlay)

(event Collision|EventActorBeginOverlap
  (params (OtherActor :type Actor%20Object%20Reference)))

(event EventTick
  (params (DeltaSeconds :type Float%20%28single-precision%29))
  (bind _fox (Variables|Default|Getfox))
  (bind _giraffe (Variables|Default|Getgiraffe))
  (Utilities|FlowControl|Sequence
    (:then_0
      (Transformation|AddWorldOffset _fox (* (Math|Vector|GetForwardVector (Variables|Default|GetfoxArrow)) 20) false false)
      (CallFunction|Check _fox))
    (:then_1
      (Transformation|AddWorldOffset _giraffe "10.000000,0.000000,0.000000" false false)
      (if (> (.x (Transformation|GetWorldLocation _giraffe)) 2e+03)
        (Transformation|SetWorldLocation _giraffe (Math|Vector|MakeVector 0.0 (Math|Random|RandomFloatinRange -1.3e+03 -2.7e+03) 1e+02) false false)))))

(fn ConstructionScript)

(fn Check
  (params (NewParam :type Skeletal%20Mesh%20Component%20Object%20Reference))
  (if (> (.y (Variables|/Script/Engine.SceneComponent|GetRelativeLocation NewParam)) (.y (Variables|/Script/Engine.SceneComponent|GetRelativeLocation (Variables|Default|GetBox))))
    (Transformation|SetRelativeLocation NewParam "0.000000,-200.000000,50.000000" false false)))