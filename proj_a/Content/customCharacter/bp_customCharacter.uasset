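; Custom character Blueprint whose Stickman skin can be painted at runtime through a render target.
; BeginPlay creates a white-cleared render target, feeds it into a dynamic skin material on Stickman, and creates a dynamic brush material.
; DrawBrush sets the brush color and draws that material onto the target's canvas, centered on a normalized location.
; BeginPlay also imports a test PNG but never uses the result.
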(event EventBeginPlay
  (Utilities|FlowControl|Sequence
    (:then_0
      (bind _returnvalue (Rendering|CreateRenderTarget2D 1024 1024 "RTF_RGBA8"))
      (bind _output_get (Variables|Default|SetrenderTarget _returnvalue))
      (Rendering|ClearRenderTarget2D _output_get "(R=1.000000,G=1.000000,B=1.000000,A=1.000000)"))
    (:then_1
      (bind _returnvalue_2 (Rendering|Material|CreateDynamicMaterialInstance "/Game/customCharacter/m_skin.m_skin" "None" "None" :!class /Script/Engine.KismetMaterialLibrary))
      (Class|KismetRenderingLibrary|ImportFileasTexture2D "test.png")
      (Rendering|Material|SetTextureParameterValue _returnvalue_2 "renderTarget" (Variables|Default|GetrenderTarget))
      (Rendering|Material|SetMaterial (Variables|Default|Getstickman) 0 _returnvalue_2))
    (:then_2
      (bind _returnvalue_3 (Rendering|Material|CreateDynamicMaterialInstance "/Game/customCharacter/m_brush.m_brush" "None" "None" :!class /Script/Engine.KismetMaterialLibrary))
      (Variables|Default|SetbrushMaterial _returnvalue_3))))

(fn ConstructionScript)

(fn DrawBrush
  (params (brushSize :type Float%20%28double-precision%29) (drawLocation :type Vector%202D%20Structure) (color :type Linear%20Color%20Structure))
  (Utilities|FlowControl|Sequence
    (:then_0
      (Rendering|Material|SetVectorParameterValue (Variables|Default|GetbrushMaterial) "brushColor" color :!class /Script/Engine.MaterialInstanceDynamic))
    (:then_1
      (bind (_canvas _size _context) (Rendering|BeginDrawCanvastoRenderTarget (Variables|Default|GetrenderTarget)))
      (Canvas|DrawMaterial :self _canvas :RenderMaterial (Variables|Default|GetbrushMaterial) :ScreenPosition (- (* _size drawLocation) (/ brushSize 2.0)) :ScreenSize (Math|Vector2D|MakeVector2D brushSize brushSize) :CoordinateSize "(X=1.000000,Y=1.000000)" :PivotPoint "(X=0.500000,Y=0.500000)")
      (Rendering|EndDrawCanvastoRenderTarget _context))))